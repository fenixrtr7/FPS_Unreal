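; AI controller for enemies that runs a behavior tree and tracks the player through AI perception.
; On BeginPlay it sets up the blackboard, seeds the target point with the pawn's location, then starts the tree.
; Each perception update for the player toggles the stored player and its blackboard key, without checking whether it was sensed.
; Waypoint patrol helpers remain, but their event-graph logic is disconnected.
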(event OnPerceptionUpdated(AIPerception)
  (params (UpdatedActors :type Array%20of%20Actor%20Object%20References))
  (for _array_element UpdatedActors
    (bind _asmy_my_character_bp (Utilities|Casting|CastToMyMyCharacterBP _array_element))
    (Utilities|IsValid (Variables|Default|GetDetectedPlayer)
      (:Is%20Valid
        (Variables|Default|SetDetectedPlayer 0)
        (Development|PrintString "Se fue")
        (AI|Components|Blackboard|ClearValue (AI|GetBlackboard self) (Variables|Default|GetDetectedPlayerName)))
      (:Is%20Not%20Valid
        (bind _output_get (Variables|Default|SetDetectedPlayer _asmy_my_character_bp))
        (Development|PrintString "Entro")
        (AI|Components|Blackboard|SetValueasObject (AI|GetBlackboard self) (Variables|Default|GetDetectedPlayerName) _output_get)))))

(event EventBeginPlay
  (bind _blackboardcomponent (Class|AIController|UseBlackboard "/Game/Blueprints/Blackboard/EnemyBlackboard.EnemyBlackboard"))
  (AI|Components|Blackboard|SetValueasVector _blackboardcomponent (Variables|Default|GetTargetPointName) (Transformation|GetActorLocation (Pawn|GetControlledPawn)))
  (AI|RunBehaviorTree "/Game/Blueprints/BehaviourTrees/enemyBehaviorTree.enemyBehaviorTree"))

(event EventTick
  (params (DeltaSeconds :type Float%20%28single-precision%29)))

(fn ConstructionScript)

(fn GetRandomTarget
  (bind _enemy (Variables|Default|GetEnemy))
  (bind _waypoints (Variables|/Game/Blueprints/EnemyBP.EnemyBP_C|GetWaypoints _enemy))
  (return (Transformation|GetActorLocation (Utilities|Array|Get(acopy) _waypoints (Math|Random|RandomIntegerinRange 0 (Utilities|Array|LastIndex _waypoints))))))

(fn ChangeTarget
  (bind _target (CallFunction|GetNextTarget))
  (bind _output_get (Variables|Default|SetTargetPosition _target))
  (AI|Navigation|MovetoLocation _output_get -1.0 true true false true 0))

(fn IsNearEnough
  (return (<= (Math|Vector|VectorLength (- (Transformation|GetActorLocation (Variables|Default|GetEnemy)) (Variables|Default|GetTargetPosition))) 1e+02)))

(fn GetNextTarget
  (bind _output_get (Variables|Default|SetCurrentWaypoint (+ (Variables|Default|GetCurrentWaypoint) 1)))
  (if (> _output_get (Utilities|Array|LastIndex (Variables|/Game/Blueprints/EnemyBP.EnemyBP_C|GetWaypoints (Variables|Default|GetEnemy))))
    (Variables|Default|SetCurrentWaypoint 0))
  (return (Transformation|GetActorLocation (Utilities|Array|Get(acopy) (Variables|/Game/Blueprints/EnemyBP.EnemyBP_C|GetWaypoints (Variables|Default|GetEnemy)) (Variables|Default|GetCurrentWaypoint)))))

(fn GoPositionPlayer
  (return (Transformation|GetActorLocation (Variables|Default|GetDetectedPlayer))))