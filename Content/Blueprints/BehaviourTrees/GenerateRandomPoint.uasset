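; Behavior tree task that picks a random point around the owning actor for AI to use.
; On execute it offsets the owner's location by an independent random value within plus or minus Range on each axis, Z included.
; It writes the result to the blackboard vector key and always finishes successfully, with no navmesh projection or reachability check.
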(event EventReceiveExecute
  (params (OwnerActor :type Actor%20Object%20Reference))
  (bind _range (Variables|Default|GetRange))
  (bind _returnvalue (* _range -1.0))
  (AI|BehaviorTree|SetBlackboardValueasVector (Variables|Default|GetValue) (+ (Transformation|GetActorLocation OwnerActor) (Math|Vector|MakeVector (Math|Random|RandomFloatinRange _returnvalue _range) (Math|Random|RandomFloatinRange _returnvalue _range) (Math|Random|RandomFloatinRange _returnvalue _range))))
  (AI|BehaviorTree|FinishExecute true))