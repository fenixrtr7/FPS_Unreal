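; Player character Blueprint with a fire input and a prototype of hitscan, per-bone damage lookup.
; The Fire action only sets the Firing flag on press and clears it on release.
; An unconnected, never-executed chain line traces forward from the camera, looks up the hit bone in the DamgesBP map and prints the value.
; BeginPlay, Tick, overlap and construction script are empty.
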(event EventBeginPlay)

(event Collision|EventActorBeginOverlap
  (params (OtherActor :type Actor%20Object%20Reference)))

(event EventTick
  (params (DeltaSeconds :type Float%20%28single-precision%29)))

(event Input|ActionEvents|InputActionFire
  (params (Key :type Key%20Structure :default "None"))
  (:Pressed
    (Variables|Default|Setfiring true))
  (:Released
    (Variables|Default|Setfiring false)))

(fn ConstructionScript)