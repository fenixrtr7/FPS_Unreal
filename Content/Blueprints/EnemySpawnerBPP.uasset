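; Enemy spawner Blueprint that fills a set of spawn points with randomly chosen actors when play begins.
; On BeginPlay it loops over every spawn point and spawns a random class from the Objetos array at that point's transform.
; A debug string prints once the loop finishes, and a leftover node for picking a random spawn point is unused.
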(event EventBeginPlay
  (bind _objetos (Variables|Default|GetObjetos))
  (for _index (range 0 (- (Utilities|Array|Length (Variables|Default|GetSpawnPoints)) 1))
    (Game|SpawnActorfromClass (Utilities|Array|Get(acopy) _objetos (Math|Random|RandomIntegerinRange 0 (- (Utilities|Array|Length _objetos) 1))) (Transformation|GetActorTransform (Utilities|Array|Get(acopy) (Variables|Default|GetSpawnPoints) _index)) "Undefined" 0 0))
  (Development|PrintString "Termino"))

(fn ConstructionScript)