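; Behavior tree task that picks the next patrol destination for an AI-controlled PatrolObjectBP pawn.
; Each execution gets the pawn's waypoints, increments an index stored on the task and wraps it to zero past the last entry.
; It writes that waypoint actor's location to a Blackboard vector key and finishes successfully, or fails if the pawn is not a PatrolObjectBP.
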(event EventReceiveExecuteAI
  (params (OwnerController :type AI%20Controller%20Object%20Reference) (ControlledPawn :type Pawn%20Object%20Reference))
  (bind _aspatrol_object_bp (Utilities|Casting|CastToPatrolObjectBP ControlledPawn)
    (:then
      (bind _waypoints (Default|GetWaypoints _aspatrol_object_bp))
      (bind _output_get (Variables|Default|SetCurrentWaypoint (+ (Variables|Default|GetCurrentWaypoint) 1)))
      (if (> _output_get (Utilities|Array|LastIndex _waypoints))
        (Variables|Default|SetCurrentWaypoint 0))
      (AI|BehaviorTree|SetBlackboardValueasVector (Variables|Default|GetBlackboard%20Value) (Transformation|GetActorLocation (Utilities|Array|Get(acopy) _waypoints (Variables|Default|GetCurrentWaypoint))))
      (AI|BehaviorTree|FinishExecute true))
    (:CastFailed
      (AI|BehaviorTree|FinishExecute false))))