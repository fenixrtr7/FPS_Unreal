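; Player character Blueprint with a hitscan weapon prototype that damages Pared actors along the shot line, with penetration.
; Fire and Fire2 inputs only toggle Firing; calls to Fire and a bone-name damage lookup are unwired.
; Fire repeats camera multi-traces with random spread, hitting each actor once per shot.
; Each Pared loses health by the current damage, then its Resistence scales damage for subsequent hits.
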(event EventBeginPlay)

(event Collision|EventActorBeginOverlap
  (params (OtherActor :type Actor%20Object%20Reference)))

(event EventTick
  (params (DeltaSeconds :type Float%20%28single-precision%29)))

(event Input|ActionEvents|InputActionFire2
  (params (Key :type Key%20Structure))
  (:Pressed
    (Variables|Default|Setfiring true))
  (:Released
    (Variables|Default|Setfiring false)))

(event Input|ActionEvents|InputActionFire
  (params (Key :type Key%20Structure))
  (:Pressed
    (Variables|Default|Setfiring true))
  (:Released
    (Variables|Default|Setfiring false)))

(fn ConstructionScript)

(fn Fire
  (params (Amount :type Integer) (Shake :type Float%20%28single-precision%29))
  (bind _returnvalue (* Shake -1.0))
  (bind _cam (Variables|Default|Getcam))
  (bind _returnvalue_2 (Transformation|GetWorldLocation _cam))
  (Variables|Default|Setfiring true)
  (for _index (range 1 Amount)
    (bind _outhits (Collision|MultiLineTraceByChannel _returnvalue_2 (+ _returnvalue_2 (* (Math|Vector|GetForwardVector _cam) 1e+04) (Math|Vector|MakeVector (Math|Random|RandomFloatinRange _returnvalue Shake) (Math|Random|RandomFloatinRange _returnvalue Shake) (Math|Random|RandomFloatinRange _returnvalue Shake))) "TraceTypeQuery3" false 0 "ForDuration"))
    (for _array_element _outhits
      (if (not (Utilities|Array|ContainsItem (Variables|Default|GetHittedObjetcs) (.HitActor (Collision|BreakHitResult _array_element))))
        (Development|PrintString (Utilities|GetDisplayName (.HitActor (Collision|BreakHitResult _array_element))))
        (Utilities|Array|Add (Variables|Default|GetHittedObjetcs) (.HitActor (Collision|BreakHitResult _array_element)))
        (bind _aspared (Utilities|Casting|CastToPared (.HitActor (Collision|BreakHitResult _array_element))))
        (bind _output_get (Variables|/Game/Pared.Pared_C|Sethealth _aspared (- (Variables|/Game/Pared.Pared_C|Gethealth _aspared) (Variables|Default|GetDamageMulti))))
        (Development|PrintString (Utilities|String|ToString(Float) _output_get))
        (Variables|Default|SetDamageMulti (* (Variables|/Game/Pared.Pared_C|GetResistence _aspared) (Variables|Default|GetDamageMulti)))))
    (Variables|Default|SetDamageMulti (Variables|Default|GetCurrentDamage))
    (Utilities|Array|Clear (Variables|Default|GetHittedObjetcs))))